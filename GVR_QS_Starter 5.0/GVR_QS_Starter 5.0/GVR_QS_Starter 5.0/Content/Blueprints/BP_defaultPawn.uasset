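; BP_defaultPawn is a pawn that detects when the camera looks at a red cube.
; Every Tick runs GazeCheck, which line-traces along the camera's forward vector on the Visibility channel with per-frame debug drawing.
; A hit that casts to BP_redCube prints a found message.
; A separate Interface event prints "Sphere" and has no caller in this graph.
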(event `self.ReceiveTick`
  (params (DeltaSeconds :type "Float (single-precision)"))
  (`self.GazeCheck`))

(event `GazeCheck`
  (bind _camera (`self.Camera`))
  (bind _returnvalue (`SceneComponent.K2_GetComponentLocation` _camera))
  ;[1 1 1] Gaze check
  (bind _outhit (`KismetSystemLibrary.LineTraceSingle` :`Start` _returnvalue :`End` (+ _returnvalue (* (`SceneComponent.GetForwardVector` _camera) 2000)) :`TraceChannel` "TraceTypeQuery1" :`DrawDebugType` "ForOneFrame"))
  (cast `/Game/Blueprints/BP_redCube` (`.HitActor` (`GameplayStatics.BreakHitResult` _outhit)))
  (`KismetSystemLibrary.PrintString` "Red Cube Found" true true (struct :`R` 1.0 :`G` 0.152464 :`B` 0.084826 :`A` 1.0)))

(event `/Game/Blueprints/NewInterface.Interface`
  (`KismetSystemLibrary.PrintString` "Sphere" true true (struct :`R` 1.0 :`G` 0.42 :`B` 0.881275 :`A` 1.0)))

(fn `UserConstructionScript`)