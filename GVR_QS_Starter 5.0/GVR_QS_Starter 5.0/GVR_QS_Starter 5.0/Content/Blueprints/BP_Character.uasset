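; BP_Character is a player character that looks with the mouse, strafes left and right, and interacts with objects under its gaze.
; Each tick, a debug-drawn Visibility line trace from the camera stores the hit actor as InteractingActor if it implements NewInterface, otherwise clears it.
; Left click sends InteractMessage to that stored actor when valid.
; A speed-scaled forward movement node exists but is unconnected.
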(event `self.ReceiveTick`
  (params (DeltaSeconds :type "Float (single-precision)"))
  (`self.GazeCheck`))

(event `InputAxis|mouseX`
  (params (AxisValue :type "Float (single-precision)"))
  ;[1 1 1] Input
  (`self.AddControllerYawInput` AxisValue))

(event `InputAxis|Move Left/Right`
  (params (AxisValue :type "Float (single-precision)"))
  ;[1 1 1] Input
  (`self.AddMovementInput` (`self.GetActorRightVector`) AxisValue))

(event `InputAxis|mouseY`
  (params (AxisValue :type "Float (single-precision)"))
  ;[1 1 1] Input
  (`self.AddControllerPitchInput` AxisValue))

(event `GazeCheck`
  (bind _camera (`self.Camera`))
  (bind _returnvalue (`SceneComponent.K2_GetComponentLocation` _camera))
  ;[1 1 1] Gaze check
  (bind _outhit (`KismetSystemLibrary.LineTraceSingle` :`Start` _returnvalue :`End` (+ _returnvalue (* (`SceneComponent.GetForwardVector` _camera) 2000)) :`TraceChannel` "TraceTypeQuery1" :`DrawDebugType` "ForOneFrame"))
  (bind (_bblockinghit _binitialoverlap _time _distance _location _impactpoint _normal _impactnormal _physmat _hitactor) (`GameplayStatics.BreakHitResult` _outhit))
  (if (`KismetSystemLibrary.DoesImplementInterface` _hitactor "/Game/Blueprints/NewInterface.NewInterface_C")
    (set `self.interactingActor` _hitactor)
    (else
      (set `self.interactingActor` null))))

(event `InputAction|Left Click`
  (params (Key :type "Key Structure"))
  (bind _interactingactor (`self.interactingActor`))
  ;[1 1 1] Partt 2 # 1
  (:`Pressed`
    (`/Engine/EditorBlueprintResources/StandardMacros.IsValid` _interactingactor
      (:`Is Valid`
        (message `/Game/Blueprints/NewInterface.Interact` _interactingactor)))))

(fn `UserConstructionScript`)